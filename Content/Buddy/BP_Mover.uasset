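; BP_Mover is an actor that slides by a set offset from its start location when enough pressure plates are active.
; PlateOn and PlateOff adjust a counter, and Latch forces it on permanently; each then calls Evaluate.
; Evaluate plays or reverses a timeline that interpolates the position through a math expression node, without sweep.
; A status light turns green when the condition is met and red otherwise.
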(event Custom|Evaluate
  (bind _startloc (Variables|Default|GetStartLoc))
  (bind _movevector (Variables|Default|GetMoveVector))
  (bind (_x _y _z) (Math|Vector|BreakVector _startloc))
  (bind (_x_2 _y_2 _z_2) (Math|Vector|BreakVector _movevector))
  (if (or (>= (Variables|Default|GetCount) (Variables|Default|GetRequired)) (Variables|Default|GetbLatched))
    (Rendering|Components|Light|SetLightColor (Variables|Default|GetStatusLight) "(R=0.1,G=1.0,B=0.2,A=1.0)" true)
    (bind _alpha (Timeline|MoveTL Play)
      (:Update
        (Transformation|SetActorLocation (|(VECT((SX+(MX*A)),(SY+(MY*A)),(SZ+(MZ*A)))) _x _x_2 _alpha _y _y_2 _z _z_2) false false)))
    (else
      (Rendering|Components|Light|SetLightColor (Variables|Default|GetStatusLight) "(R=1.0,G=0.1,B=0.1,A=1.0)" true)
      (Timeline|MoveTL Reverse))))

(event Custom|PlateOn
  (Variables|Default|SetCount (+ (Variables|Default|GetCount) 1))
  (CallFunction|Evaluate))

(event Custom|PlateOff
  (Variables|Default|SetCount (- (Variables|Default|GetCount) 1))
  (CallFunction|Evaluate))

(event Custom|Latch
  (Variables|Default|SetbLatched true)
  (CallFunction|Evaluate))

(event EventBeginPlay
  (Variables|Default|SetStartLoc (Transformation|GetActorLocation)))

(event Collision|EventActorBeginOverlap
  (params (OtherActor :type Actor%20Object%20Reference)))

(event EventTick
  (params (DeltaSeconds :type Float%20%28single-precision%29)))

(fn ConstructionScript)