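; BP_GoalTrigger is a level goal pad that shows the victory screen when the first-person character overlaps it.
; On BeginPlay it tints the Pad mesh gold through a dynamic material instance.
; The first valid overlap sets a Done flag, adds WBP_Victory to the viewport, switches to UI-only input with a visible cursor and pauses the game.
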(event EventBeginPlay
  (bind _returnvalue (Rendering|Material|CreateDynamicMaterialInstance (Variables|Default|GetPad) 0 0 "None" :!class /Script/Engine.PrimitiveComponent))
  (Rendering|Material|SetVectorParameterValue _returnvalue "Color" "(R=0.6,G=0.4,B=0.03,A=1.0)" :!class /Script/Engine.MaterialInstanceDynamic))

(event Collision|EventActorBeginOverlap
  (params (OtherActor :type Actor%20Object%20Reference))
  (bind _returnvalue (Game|GetPlayerController 0))
  (Utilities|Casting|CastToBP_FirstPersonCharacter OtherActor)
  (if (not (Variables|Default|GetbDone))
    (Variables|Default|SetbDone true)
    (bind _returnvalue_2 (UserInterface|CreateWidget "/Game/Buddy/WBP_Victory.WBP_Victory_C" _returnvalue))
    (UserInterface|Viewport|AddtoViewport _returnvalue_2 0)
    (Variables|/Script/Engine.PlayerController|SetbShowMouseCursor _returnvalue true)
    (Input|SetInputModeUIOnly _returnvalue _returnvalue_2 "DoNotLock" false)
    (Game|SetGamePaused true)))

(event EventTick
  (params (DeltaSeconds :type Float%20%28single-precision%29)))

(fn ConstructionScript)