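; Checkpoint actor that saves a respawn point on the first-person character the first time it overlaps.
; BeginPlay tints the Pad with a dynamic material instance.
; The overlap sets a one-time Reached flag and writes the character's RespawnLocation as the checkpoint position raised slightly in Z.
; Unless Silent is set, it shows a WBP_Toast widget, then removes it after a short delay.
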(event EventBeginPlay
  (bind _returnvalue (Rendering|Material|CreateDynamicMaterialInstance (Variables|Default|GetPad) 0 0 "None" :!class /Script/Engine.PrimitiveComponent))
  (Rendering|Material|SetVectorParameterValue _returnvalue "Color" "(R=0.02,G=0.35,B=0.28,A=1.0)" :!class /Script/Engine.MaterialInstanceDynamic))

(event Collision|EventActorBeginOverlap
  (params (OtherActor :type Actor%20Object%20Reference))
  (bind _returnvalue (Transformation|GetActorLocation))
  (bind (_x _y _z) (Math|Vector|BreakVector _returnvalue))
  (bind _asbp_first_person_character (Utilities|Casting|CastToBP_FirstPersonCharacter OtherActor))
  (if (not (Variables|Default|GetbReached))
    (Variables|Default|SetbReached true)
    (Variables|/Game/FirstPerson/Blueprints/BP_FirstPersonCharacter.BP_FirstPersonCharacter_C|SetRespawnLocation _asbp_first_person_character (|(VECT(CX,CY,(CZ+110))) _x _y _z))
    (if (not (Variables|Default|GetSilent))
      (bind _returnvalue_2 (UserInterface|CreateWidget "/Game/Buddy/WBP_Toast.WBP_Toast_C" (Game|GetPlayerController 0)))
      (Variables|Default|SetToastRef _returnvalue_2)
      (UserInterface|Viewport|AddtoViewport (Variables|Default|GetToastRef) 0)
      (Utilities|FlowControl|Delay 2.5)
      (Widget|RemovefromParent (Variables|Default|GetToastRef)))))

(event EventTick
  (params (DeltaSeconds :type Float%20%28single-precision%29)))

(fn ConstructionScript)