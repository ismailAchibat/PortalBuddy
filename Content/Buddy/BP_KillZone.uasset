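; BP_KillZone is a kill volume that recovers the first-person player and the Buddy companion when they overlap it.
; The player teleports to the respawn location stored on their character.
; Buddy teleports to a fixed offset beside and above the player's current position, computed by a Math Expression node.
; Both have their movement stopped immediately after teleporting, so no velocity carries over.
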(event EventBeginPlay)

(event Collision|EventActorBeginOverlap
  (params (OtherActor :type Actor%20Object%20Reference))
  (bind _asbp_first_person_character (Utilities|Casting|CastToBP_FirstPersonCharacter OtherActor)
    (:then
      (Transformation|SetActorLocation _asbp_first_person_character (Variables|/Game/FirstPerson/Blueprints/BP_FirstPersonCharacter.BP_FirstPersonCharacter_C|GetRespawnLocation _asbp_first_person_character) false true)
      (Components|Movement|StopMovementImmediately (Variables|/Script/Engine.Character|GetCharacterMovement _asbp_first_person_character)))
    (:CastFailed
      (bind _asbp_buddy (Utilities|Casting|CastToBP_Buddy OtherActor))
      (bind _returnvalue (Actor|GetActorOfClass "/Game/FirstPerson/Blueprints/BP_FirstPersonCharacter.BP_FirstPersonCharacter_C"))
      (Transformation|SetActorLocation _asbp_buddy (|(VECT((PX+150),PY,(PZ+100))) (.X (Math|Vector|BreakVector (Transformation|GetActorLocation _returnvalue))) (.Y (Math|Vector|BreakVector (Transformation|GetActorLocation _returnvalue))) (.Z (Math|Vector|BreakVector (Transformation|GetActorLocation _returnvalue)))) false true)
      (Components|Movement|StopMovementImmediately (Variables|/Script/Engine.Character|GetCharacterMovement _asbp_buddy)))))

(event EventTick
  (params (DeltaSeconds :type Float%20%28single-precision%29)))

(fn ConstructionScript)