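; BP_PlateLight is a pressure plate actor that responds only to BP_Buddy.
; When the buddy begins or ends overlap, it calls PlateOn or PlateOff on TargetRef and switches StatusLight between green and light blue.
; At BeginPlay it creates a dynamic material on the Plate mesh and tints it dark blue; that color does not change afterward.
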(event EventBeginPlay
  (bind _returnvalue (Rendering|Material|CreateDynamicMaterialInstance (Variables|Default|GetPlate) 0 0 "None" :!class /Script/Engine.PrimitiveComponent))
  (Rendering|Material|SetVectorParameterValue _returnvalue "Color" "(R=0.05,G=0.25,B=0.6,A=1.0)" :!class /Script/Engine.MaterialInstanceDynamic))

(event Collision|EventActorBeginOverlap
  (params (OtherActor :type Actor%20Object%20Reference))
  (Utilities|Casting|CastToBP_Buddy OtherActor)
  (Default|Plateon (Variables|Default|GetTargetRef))
  (Rendering|Components|Light|SetLightColor (Variables|Default|GetStatusLight) "(R=0.1,G=1.0,B=0.2,A=1.0)" true))

(event EventTick
  (params (DeltaSeconds :type Float%20%28single-precision%29)))

(event Collision|EventActorEndOverlap
  (params (OtherActor :type Actor%20Object%20Reference))
  (Utilities|Casting|CastToBP_Buddy OtherActor)
  (Default|PlateOff (Variables|Default|GetTargetRef))
  (Rendering|Components|Light|SetLightColor (Variables|Default|GetStatusLight) "(R=0.24,G=0.63,B=1.0,A=1.0)" true))

(fn ConstructionScript)