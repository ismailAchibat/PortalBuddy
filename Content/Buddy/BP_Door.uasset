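; BP_Door is a door actor that turns its status light green and rises vertically when OpenDoor is called.
; BeginPlay caches the starting location, and the DoorTL timeline alpha drives a math expression that offsets Z by up to 400 units, assuming a 0–1 curve.
; Movement teleports without sweeping, and the file contains no closing logic or overlap trigger.
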(event Custom|OpenDoor
  (bind _startloc (Variables|Default|GetStartLoc))
  (bind (_x _y _z) (Math|Vector|BreakVector _startloc))
  (Rendering|Components|Light|SetLightColor (Variables|Default|GetStatusLight) "(R=0.1,G=1.0,B=0.2,A=1.0)" true)
  (bind _alpha (Timeline|DoorTL PlayFromStart)
    (:Update
      (Transformation|SetActorLocation (|(VECT(SX,SY,(SZ+(A*400)))) _x _y _z _alpha) false true))))

(event EventBeginPlay
  (Variables|Default|SetStartLoc (Transformation|GetActorLocation)))

(event Collision|EventActorBeginOverlap
  (params (OtherActor :type Actor%20Object%20Reference)))

(event EventTick
  (params (DeltaSeconds :type Float%20%28single-precision%29)))

(fn ConstructionScript)